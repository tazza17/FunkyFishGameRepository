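; FunkyFish_Character is a player character with movement, camera controls and selectable potions.
; H and L set the held potion class to healing or fire, and left click spawns it slightly above the character.
; Enhanced Input drives walking and mouse look, while raw keys handle jump, crouch, sprint with a wider FOV, and a third/first-person camera toggle.
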(event `Key|LeftMouseButton`
  (params (Key :type "Key Structure"))
  ;[1 1 1 0.5] Potions Code :)
  (:`Pressed`
    (`self.SwitchPotion`)))

(event `Key|H`
  (params (Key :type "Key Structure"))
  ;[1 1 1 0.5] Potions Code :)
  (:`Pressed`
    (set `self.CurrentHeldPotion` "/Game/Blueprints/Potions/BP_Potion_Healing.BP_Potion_Healing_C")))

(event `Key|L`
  (params (Key :type "Key Structure"))
  ;[1 1 1 0.5] Potions Code :)
  (:`Pressed`
    (set `self.CurrentHeldPotion` "/Game/Blueprints/Potions/BP_Potion_Fire.BP_Potion_Fire_C")))

(event `SwitchPotion`
  (bind _returnvalue (`self.GetTransform`))
  ;[1 1 1 0.5] Potions Code :)
  (`|SpawnActorFromClass` (`self.CurrentHeldPotion`) (`KismetMathLibrary.MakeTransform` (`KismetMathLibrary.MakeVector` (.x (.location _returnvalue)) (.y (.location _returnvalue)) (+ (.z (.location _returnvalue)) 60.0)) (.rotation _returnvalue) (.scale _returnvalue)) "AlwaysSpawn" "MultiplyWithRoot" null null))

(event `self.ReceiveBeginPlay`
  ;[1 0 0.6972 0.5] Mapping context
  (`EnhancedInputSubsystemInterface.AddMappingContext` (pcsubsystem `EnhancedInputLocalPlayerSubsystem` (`GameplayStatics.GetPlayerController` 0)) "/Game/Blueprints/controls/IMCC.IMCC" 0 (struct)))

(event `EnhancedInput|/Game/Blueprints/controls/IA_WASD`
  (params (ActionValue :type "Vector2D Structure") (ElapsedSeconds :type "Float (double-precision)") (TriggeredSeconds :type "Float (double-precision)") (InputAction :type "InputAction Object Reference" :default "/Game/Blueprints/controls/IA_WASD.IA_WASD"))
  (bind (_returnvalue_x _returnvalue_y) (`KismetMathLibrary.BreakVector2D` (`|GetInputActionValue`)))
  ;[0.05159 0 1 0.5 30] MOVEMENTS
  (:`Triggered`
    (`self.AddMovementInput` (`self.GetActorRightVector`) _returnvalue_x)
    (`self.AddMovementInput` (`self.GetActorForwardVector`) _returnvalue_y)))

(event `Key|SpaceBar`
  (params (Key :type "Key Structure"))
  ;[0.05159 0 1 0.5 30] MOVEMENTS
  (:`Pressed`
    (`self.Jump`)))

(event `Key|LeftShift`
  (params (Key :type "Key Structure"))
  (bind _charactermovement (`self.CharacterMovement`))
  ;[0.05159 0 1 0.5 30] MOVEMENTS
  (:`Pressed`
    (set `CharacterMovementComponent.MaxWalkSpeed` 1800.0 _charactermovement)
    (`CameraComponent.SetFieldOfView` (`self.Camera`) 107.0))
  (:`Released`
    (set `CharacterMovementComponent.MaxWalkSpeed` 600.0 _charactermovement)
    (`CameraComponent.SetFieldOfView` (`self.Camera`) 90.0)))

(event `Key|G`
  (params (Key :type "Key Structure"))
  (bind _camera (`self.Camera`))
  (:`Pressed`
    (`/Engine/EditorBlueprintResources/StandardMacros.FlipFlop`
      (:`A`
        (`SceneComponent.K2_SetRelativeLocationAndRotation` _camera (-264.696498 0.0 145.006911) (struct :`Pitch` -20.0) false false))
      (:`B`
        (`SceneComponent.K2_SetRelativeLocationAndRotation` :`self` _camera :`NewLocation` (0.0 0.0 60.0))))))

(event `EnhancedInput|/Game/Blueprints/controls/IA_Mouse`
  (params (ActionValue :type "Vector2D Structure") (ElapsedSeconds :type "Float (double-precision)") (TriggeredSeconds :type "Float (double-precision)") (InputAction :type "InputAction Object Reference" :default "/Game/Blueprints/controls/IA_Mouse.IA_Mouse"))
  ;[0.05159 0 1 0.5 30] MOVEMENTS
  (:`Triggered`
    (`self.AddControllerYawInput` ActionValue_X)
    (`self.AddControllerPitchInput` (* ActionValue_Y -1.0))))

(event `Key|LeftControl`
  (params (Key :type "Key Structure"))
  ;[0.05159 0 1 0.5 30] MOVEMENTS
  (:`Pressed`
    (`self.Crouch`))
  (:`Released`
    (`self.UnCrouch`)))

(fn `UserConstructionScript`)