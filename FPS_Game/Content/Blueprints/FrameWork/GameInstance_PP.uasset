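; GameInstance_PP is a game instance Blueprint that picks a random chest loot item for a requested rarity.
; GetChestItem filters LootpoolArray by rarity into ItemsOfRarity, shuffles that list and returns the first entry's pickup actor.
; It prints the rarity on each call and does not check for an empty match list before reading the first element.
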(fn `GetChestItem`
  (params (Rarity :type Integer))
  (returns (ItemReceived :type "/Game/Blueprints/Actors/Pickups/BP_PickUp Class Reference"))
  (bind _itemsofrarity (`self.ItemsOfRarity`))
  (bind _output_pickupactor (break `/Game/Blueprints/FrameWork/S_Lootpool` (`|GetArrayItem` _itemsofrarity)))
  (`KismetSystemLibrary.PrintString` (`KismetStringLibrary.Conv_IntToString` Rarity))
  (`KismetArrayLibrary.Array_Clear` (`self.ItemsOfRarity`))
  (for _array_element (`self.Lootpool Array`)
    (if (== (`.RarityLevel1-3_6_B1F8B1F545B008D9B83D668F31306022` (break `/Game/Blueprints/FrameWork/S_Lootpool` _array_element)) Rarity)
      (`KismetArrayLibrary.Array_Add` (`self.ItemsOfRarity`) _array_element)))
  (`KismetArrayLibrary.Array_Shuffle` _itemsofrarity)
  (return _output_pickupactor))