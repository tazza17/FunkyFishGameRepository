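; Player character Blueprint that handles movement and potion throwing.
; Enhanced Input drives walking, look and throw, while hard-wired keys handle jump, crouch, sprint with wider FOV, and a toggle between two camera placements.
; Number keys select the normal, fire or healing potion class, which the throw spawns at HeldObject.
; A timer gates throws by cooldown, and each throw passes that cooldown to the HUD.
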(event `self.ReceiveBeginPlay`
  ;[1 0 0.6972 0.5] Mapping context
  (`EnhancedInputSubsystemInterface.AddMappingContext` (pcsubsystem `EnhancedInputLocalPlayerSubsystem` (`GameplayStatics.GetPlayerController` 0)) "/Game/Blueprints/Inputs/InputMappingContext_PP.InputMappingContext_PP" 0 (struct)))

(event `EnhancedInput|/Game/Blueprints/Inputs/IA_WASD`
  (params (ActionValue :type "Vector2D Structure") (ElapsedSeconds :type "Float (double-precision)") (TriggeredSeconds :type "Float (double-precision)") (InputAction :type "InputAction Object Reference" :default "/Game/Blueprints/Inputs/IA_WASD.IA_WASD"))
  (bind (_returnvalue_x _returnvalue_y) (`KismetMathLibrary.BreakVector2D` (`|GetInputActionValue`)))
  ;[0.05159 0 1 0.5 30] MOVEMENTS
  (:`Triggered`
    (`self.AddMovementInput` (`self.GetActorRightVector`) _returnvalue_x)
    (`self.AddMovementInput` (`self.GetActorForwardVector`) _returnvalue_y)))

(event `Key|LeftControl`
  (params (Key :type "Key Structure"))
  ;[0.05159 0 1 0.5 30] MOVEMENTS
  (:`Pressed`
    (`self.Crouch`))
  (:`Released`
    (`self.UnCrouch`)))

(event `Key|G`
  (params (Key :type "Key Structure"))
  (bind _camera (`self.Camera`))
  (:`Pressed`
    (`/Engine/EditorBlueprintResources/StandardMacros.FlipFlop`
      (:`A`
        (`SceneComponent.K2_SetRelativeLocationAndRotation` _camera (-264.696498 0.0 145.006911) (struct :`Pitch` -20.0) false false))
      (:`B`
        (`SceneComponent.K2_SetRelativeLocationAndRotation` :`self` _camera :`NewLocation` (0.0 0.0 60.0))))))

(event `Key|SpaceBar`
  (params (Key :type "Key Structure"))
  ;[0.05159 0 1 0.5 30] MOVEMENTS
  (:`Pressed`
    (`self.Jump`)))

(event `EnhancedInput|/Game/Blueprints/Inputs/IA_Mouse`
  (params (ActionValue :type "Vector2D Structure") (ElapsedSeconds :type "Float (double-precision)") (TriggeredSeconds :type "Float (double-precision)") (InputAction :type "InputAction Object Reference" :default "/Game/Blueprints/Inputs/IA_Mouse.IA_Mouse"))
  ;[0.05159 0 1 0.5 30] MOVEMENTS
  (:`Triggered`
    (`self.AddControllerYawInput` ActionValue_X)
    (`self.AddControllerPitchInput` (* ActionValue_Y -1.0))))

(event `Key|LeftShift`
  (params (Key :type "Key Structure"))
  (bind _charactermovement (`self.CharacterMovement`))
  (bind _camera (`self.Camera`))
  ;[0.05159 0 1 0.5 30] MOVEMENTS
  (:`Pressed`
    (set `CharacterMovementComponent.MaxWalkSpeed` 1800.0 _charactermovement)
    (`CameraComponent.SetFieldOfView` _camera 107.0))
  (:`Released`
    (set `CharacterMovementComponent.MaxWalkSpeed` 600.0 _charactermovement)
    (`CameraComponent.SetFieldOfView` _camera 90.0)))

(event `Key|One`
  (params (Key :type "Key Structure"))
  ;[1 1 1 0.5] Potions Code :)
  (:`Pressed`
    (set `self.CurrentHeldPotion` "/Game/Blueprints/Actors/Potions/BP_Potion.BP_Potion_C")))

(event `Key|Two`
  (params (Key :type "Key Structure"))
  ;[1 1 1 0.5] Potions Code :)
  (:`Pressed`
    (set `self.CurrentHeldPotion` "/Game/Blueprints/Actors/Potions/BP_Potion_Fire.BP_Potion_Fire_C")))

(event `Key|Three`
  (params (Key :type "Key Structure"))
  ;[1 1 1 0.5] Potions Code :)
  (:`Pressed`
    (set `self.CurrentHeldPotion` "/Game/Blueprints/Actors/Potions/BP_Potion_Healing.BP_Potion_Healing_C")))

(event `EnhancedInput|/Game/Blueprints/Inputs/IA_Throw`
  (params (ActionValue :type Boolean) (ElapsedSeconds :type "Float (double-precision)") (TriggeredSeconds :type "Float (double-precision)") (InputAction :type "InputAction Object Reference" :default "/Game/Blueprints/Inputs/IA_Throw.IA_Throw"))
  (bind _heldobject (`self.HeldObject`))
  (bind _throwcooldown (`self.ThrowCooldown`))
  (bind (_returnvalue_x _returnvalue_y _returnvalue_z) (`KismetMathLibrary.BreakVector` (`SceneComponent.K2_GetComponentLocation` _heldobject)))
  ;[1 1 1 0.5] Potions Code :)
  (:`Triggered`
    (if (`self.CanThrow?`)
      (set `self.CanThrow?` false)
      (`|SpawnActorFromClass` (`self.CurrentHeldPotion`) (`KismetMathLibrary.MakeTransform` (`KismetMathLibrary.MakeVector` _returnvalue_x _returnvalue_y _returnvalue_z) (`SceneComponent.K2_GetComponentRotation` _heldobject)) "AlwaysSpawn" "MultiplyWithRoot" null null)
      (`KismetSystemLibrary.K2_SetTimerDelegate` (delegate `CooldownFinish`) _throwcooldown)
      (bind _ashud_pp (cast `/Game/Blueprints/FrameWork/HUD_PP` (`PlayerController.GetHUD` (`GameplayStatics.GetPlayerController` 0))))
      (`/Game/Blueprints/Widgets/WBP_HUD.PotionThrown` (`/Game/Blueprints/FrameWork/HUD_PP.HUDREF` _ashud_pp) _throwcooldown))))

(event `CooldownFinish`
  ;[1 1 1 0.5] Potions Code :)
  (set `self.CanThrow?` true))

(fn `UserConstructionScript`)